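; Base actor with health, a floating health bar and a destroyed state, apparently a structure to defend or attack.
; A BeginPlay loop refreshes the HealthGreen widget's percentage every 0.1 seconds and yaws it toward the player camera.
; SetHealth subtracts damage, then tests the new health minus that damage again.
; At zero or below, it destroys the collision sphere and reveals a particle effect.
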(event `self.ReceiveBeginPlay`
  (bind _ashealth_green (cast `/Game/base/Blueprints/HealthGreen` (`WidgetComponent.GetUserWidgetObject` (`self.Health`))))
  (`ProgressBar.SetPercent` (`/Game/base/Blueprints/HealthGreen.ProgressBar_156` _ashealth_green) (/ (`self.current_health`) (`self.max_health`)) :!label _label)
  (`SceneComponent.K2_SetWorldRotation` (`self.Health`) (`KismetMathLibrary.MakeRotator` 0.0 0.0 (.yaw (`KismetMathLibrary.FindLookAtRotation` (`SceneComponent.K2_GetComponentLocation` (`self.Health`)) (`PlayerCameraManager.GetCameraLocation` (`GameplayStatics.GetPlayerCameraManager` 0))))) false false)
  (`KismetSystemLibrary.Delay` 0.1)
  (goto _label))

(fn `SetHealth`
  (params (Resta :type "Float (double-precision)"))
  (bind _spherecollision (`self.SphereCollision`))
  (bind _returnvalue (- (`self.current_health`) Resta))
  (set `self.current_health` _returnvalue)
  (if (<= _returnvalue 0.0)
    (`/Engine/EditorBlueprintResources/StandardMacros.IsValid` _spherecollision
      (:`Is Valid`
        (`ActorComponent.K2_DestroyComponent` _spherecollision)
        (`SceneComponent.SetVisibility` (`self.ParticleSystem1`) true false)))))

(fn `UserConstructionScript`)